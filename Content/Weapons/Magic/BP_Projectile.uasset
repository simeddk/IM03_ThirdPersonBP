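; BP_Projectile is a magic projectile, owned by a BP_Skill_Throw, that destroys itself after a short lifespan.
; Helper functions walk the ownership chain from the throw skill to its magic and that magic's owner.
; SendDamage ignores that owner, spawns an impact emitter rotated along the owner-to-target direction, forwards damage to the magic, then destroys the projectile.
; It has no movement or active overlap logic in its own graphs.
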(event EventBeginPlay
  (Actor|SetLifeSpan 5.0))

(event Collision|EventActorBeginOverlap
  (params (OtherActor :type Actor%20Object%20Reference)))

(event EventTick
  (params (DeltaSeconds :type Float%20%28single-precision%29)))

(fn ConstructionScript)

(fn GetOwnertoSkillThrow
  (bind _asbp_skill_throw (Utilities|Casting|CastToBP_Skill_Throw (Components|GetOwner)))
  (return _asbp_skill_throw))

(fn GetOwnertoMagic
  (return (Default|GetOwnertoMagic (CallFunction|GetOwnertoSkillThrow))))

(fn SendDamage
  (params (OtherActor :type Actor%20Object%20Reference) (Damage :type Float%20%28single-precision%29) (ImpactParticle :type Particle%20System%20Object%20Reference) (ImpactLocation :type Vector) (ImpactScale :type Vector :default "1.000000,1.000000,1.000000"))
  (if (!= OtherActor (Components|GetOwner (CallFunction|GetOwnertoMagic)))
    (Effects|SpawnEmitteratLocation ImpactParticle (+ (Transformation|GetActorLocation) ImpactLocation) (Math|Rotator|FindLookatRotation (Transformation|GetActorLocation (Components|GetOwner (CallFunction|GetOwnertoMagic))) (Transformation|GetActorLocation OtherActor)) ImpactScale)
    (Default|SendDamage (CallFunction|GetOwnertoMagic) OtherActor Damage)
    (Actor|DestroyActor)))