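; BP_Skill_Heal is a magic skill that heals its caster through the owner's StatusComponent.
; Spell checks that health is below maximum, then adds HealAmount, disables movement through the owning magic object and plays a buff montage.
; At full health it prints a debug message and calls Spelled immediately.
; Spelled re-enables movement; after a successful heal, this file does not call it itself.
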(event EventSpell
  (bind _ascharacter (CallFunction|GetOwnertoCharacter))
  (bind _returnvalue (Actor|GetComponentbyClass _ascharacter "/Game/Components/StatusComponent.StatusComponent_C"))
  (|CallParentFunction)
  (Utilities|IsValid _returnvalue
    (:Is%20Valid
      (if (< (Variables|/Game/Components/StatusComponent.StatusComponent_C|GetHealth _returnvalue) (Variables|/Game/Components/StatusComponent.StatusComponent_C|GetMaxHealth _returnvalue))
        (Default|IncreaseHealth _returnvalue (Variables|Default|GetHealAmount))
        (Default|SetStateMove (CallFunction|GetOwnertoMagic) false)
        (Animation|PlayAnimMontage (CallFunction|GetOwnertoCharacter) "/Game/Character/Animations/Magic/MG_Buff_Montage.MG_Buff_Montage" 1.0 "None")
        (else
          (Development|PrintString "이미 체력이 꽉참")
          (CallFunction|Spelled))))))

(event EventSpelled
  (|CallParentFunction)
  (Default|SetStateMove (CallFunction|GetOwnertoMagic) true))

(fn ConstructionScript
  (|CallParentFunction))