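; BP_Fist is an unarmed melee weapon whose punches and kicks damage what they touch.
; On BeginPlay it attaches four limb collision components to sockets on the owning Character's mesh and disables all sphere collisions.
; OnCollision enables the component for the requested limb, and OffCollision disables all spheres again.
; Each overlap sends damage from DamageComponent, based on the current combo count.
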(event OnComponentBeginOverlap(LeftPunch)
  (params (OverlappedComponent :type Primitive%20Component%20Object%20Reference) (OtherActor :type Actor%20Object%20Reference) (OtherComp :type Primitive%20Component%20Object%20Reference) (OtherBodyIndex :type Integer) (bFromSweep :type Boolean) (SweepResult :type Hit%20Result%20Structure%20%28by%20ref%29))
  (CallFunction|SendDamage OtherActor (Default|GetDamage (Variables|Default|GetDamageComponent) (Variables|Default|GetComboCount))))

(event OnComponentBeginOverlap(RgihtPunch)
  (params (OverlappedComponent :type Primitive%20Component%20Object%20Reference) (OtherActor :type Actor%20Object%20Reference) (OtherComp :type Primitive%20Component%20Object%20Reference) (OtherBodyIndex :type Integer) (bFromSweep :type Boolean) (SweepResult :type Hit%20Result%20Structure%20%28by%20ref%29))
  (CallFunction|SendDamage OtherActor (Default|GetDamage (Variables|Default|GetDamageComponent) (Variables|Default|GetComboCount))))

(event OnComponentBeginOverlap(LeftKick)
  (params (OverlappedComponent :type Primitive%20Component%20Object%20Reference) (OtherActor :type Actor%20Object%20Reference) (OtherComp :type Primitive%20Component%20Object%20Reference) (OtherBodyIndex :type Integer) (bFromSweep :type Boolean) (SweepResult :type Hit%20Result%20Structure%20%28by%20ref%29))
  (CallFunction|SendDamage OtherActor (Default|GetDamage (Variables|Default|GetDamageComponent) (Variables|Default|GetComboCount))))

(event OnComponentBeginOverlap(RightKick)
  (params (OverlappedComponent :type Primitive%20Component%20Object%20Reference) (OtherActor :type Actor%20Object%20Reference) (OtherComp :type Primitive%20Component%20Object%20Reference) (OtherBodyIndex :type Integer) (bFromSweep :type Boolean) (SweepResult :type Hit%20Result%20Structure%20%28by%20ref%29))
  (CallFunction|SendDamage OtherActor (Default|GetDamage (Variables|Default|GetDamageComponent) (Variables|Default|GetComboCount))))

(event EventBeginPlay
  (|CallParentFunction)
  (Utilities|FlowControl|Sequence
    (:then_0
      (CallFunction|AttachCollisiontoSocket (Variables|Default|GetLeftPunch) "Fist_LeftPunch")
      (CallFunction|AttachCollisiontoSocket (Variables|Default|GetRgihtPunch) "Fist_RightPunch"))
    (:then_1
      (CallFunction|AttachCollisiontoSocket (Variables|Default|GetLeftKick) "Fist_LeftKick")
      (CallFunction|AttachCollisiontoSocket (Variables|Default|GetRightKick) "Fist_RightKick")
      (CallFunction|SetAllCollisions "NoCollision"))))

(event EventOnCollision
  (params (DesiredCollision :type EFistType%20Enum :default "NewEnumerator0"))
  (|CallParentFunction DesiredCollision)
  (switch Utilities|FlowControl|Switch|SwitchonEFistType DesiredCollision
    (:NewEnumerator1
      (Collision|SetCollisionEnabled (Variables|Default|GetLeftPunch) "QueryAndPhysics"))
    (:NewEnumerator2
      (Collision|SetCollisionEnabled (Variables|Default|GetRgihtPunch) "QueryAndPhysics"))
    (:NewEnumerator3
      (Collision|SetCollisionEnabled (Variables|Default|GetLeftKick) "QueryAndPhysics"))
    (:NewEnumerator4
      (Collision|SetCollisionEnabled (Variables|Default|GetRightKick) "QueryAndPhysics"))))

(event EventOffCollision
  (|CallParentFunction)
  (CallFunction|SetAllCollisions "NoCollision"))

(fn ConstructionScript)

(fn AttachCollisiontoSocket
  (params (Collision :type Sphere%20Component%20Object%20Reference) (SocketName :type Name))
  (bind _ascharacter (Utilities|Casting|CastToCharacter (Components|GetOwner)))
  (Transformation|AttachComponentToComponent Collision (Variables|/Script/Engine.Character|GetMesh _ascharacter) SocketName "KeepRelative" "KeepRelative" "KeepRelative" true))

(fn SetAllCollisions
  (params (CollisionType :type ECollisionEnabled%20Enum :default "NoCollision"))
  (for _array_element (Actor|GetComponentsByClass "/Script/Engine.SphereComponent")
    (Collision|SetCollisionEnabled _array_element CollisionType)))