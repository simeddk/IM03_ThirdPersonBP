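; BP_Melee is a melee weapon that plays combo attacks from DataTable montage rows matching its MeleeType, loaded on BeginPlay.
; Attack starts the chain or, during the combo window, queues the next step for NextCombo, while EndAction resets state.
; SendDamage hits each actor once until OffCollision clears the list.
; Successful hits trigger camera shake and brief time-dilation hit stop, plus a particle effect on the final combo hit.
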(event Custom|DamageEffect
  (Utilities|FlowControl|Sequence
    (:then_0
      (if (Variables|Default|GetbLastCombo)
        (Effects|SpawnEmitteratLocation (Variables|Default|GetLastComboEffect) (Transformation|GetActorLocation))))
    (:then_1
      (Class|PlayerController|ClientPlayCameraShake (Game|GetPlayerController 0) "/Game/Weapons/Melee/Shake_Hit.Shake_Hit_C" 1.0 "CameraLocal" "0, 0, 0")
      (Utilities|Time|SetGlobalTimeDilation 0.15)
      (Utilities|FlowControl|Delay 0.02)
      (Utilities|Time|SetGlobalTimeDilation 1.0))))

(event Custom|NextCombo
  ;[1 1 1] 콤보 연결 성공 시
  (if (Variables|Default|GetbSucceedCombo)
    (Variables|Default|SetbSucceedCombo false)
    (Math|Integer|IncrementInt (Variables|Default|GetComboCount)
      (:%20%20
        (CallFunction|PlayComboMontage)
        (Variables|Default|SetbLastCombo (== (Variables|Default|GetComboCount) (- (Utilities|Array|Length (Variables|Default|GetMeleeDatas)) 1)))))))

(event EventEndAction
  ;[1 1 1] 막타 or 콤보 실패 시
  (|CallParentFunction)
  (CallFunction|SetStateIdling)
  (CallFunction|SetStateMove true)
  (Variables|Default|SetComboCount 0)
  (Variables|Default|SetbCanCombo false)
  (Variables|Default|SetbSucceedCombo false)
  (Variables|Default|SetbLastCombo false))

(event EventAttack
  ;[1 1 1] 왼클릭 시
  (|CallParentFunction)
  (if (Variables|Default|GetbCanCombo)
    (Variables|Default|SetbCanCombo false)
    (Variables|Default|SetbSucceedCombo true)
    (elif (CallFunction|CanAttack)
      (CallFunction|SetStateAttacking)
      (CallFunction|PlayComboMontage))))

(event EventBeginPlay
  ;[1 1 1] Read DataTable
  (|CallParentFunction)
  (bind _outrownames (DataTable|GetDataTableRowNames (Variables|Default|GetDataTable)))
  (for _array_element _outrownames
    (bind _returnvalue (Utilities|GetDataTableRow (Variables|Default|GetDataTable) _array_element)
      (:then
        (if (Utilities|Enum|Equal(Enum) (.MeleeType (Utilities|Struct|BreakFMeleeData _returnvalue)) (Variables|Default|GetMeleeType))
          (Utilities|Array|Add (Variables|Default|GetMeleeDatas) _returnvalue))))))

(fn ConstructionScript
  (|CallParentFunction))

(fn PlayComboMontage
  (bind _meleedatas (Variables|Default|GetMeleeDatas))
  (bind _combocount (Variables|Default|GetComboCount))
  (bind _output (Utilities|Array|Get(acopy) _meleedatas _combocount))
  (bind _ascharacter (Utilities|Casting|CastToCharacter (Components|GetOwner)))
  (Animation|PlayAnimMontage _ascharacter (.animmontage _output) (.playrate _output) (.startsection _output))
  (CallFunction|SetStateMove (.bcanmove _output)))

(fn OnCollision
  (params (DesiredCollision :type EFistType%20Enum :default "NewEnumerator0")))

(fn OffCollision
  (Utilities|Array|Clear (Variables|Default|GetHittedActors)))

(fn SendDamage
  (params (OtherActor :type Actor%20Object%20Reference) (Damage :type Float%20%28single-precision%29))
  (bind _array_element (Utilities|Array|ForEachLoopwithBreak (Variables|Default|GetHittedActors) :!label _label)
    (:LoopBody
      (if (== _array_element OtherActor)
        (LocalVariables|SetbEverHittedActor true)
        (goto _label Break)))
    (:Completed
      (if (not (LocalVariables|GetbEverHittedActor))
        (Utilities|Array|Add (Variables|Default|GetHittedActors) OtherActor)
        (bind _bresult (|CallParentFunction OtherActor Damage))
        (if _bresult
          (CallFunction|DamageEffect)
          (return _bresult))))))